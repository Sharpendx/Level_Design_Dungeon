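; DanPuzzle_BP is a puzzle room that shuts the player in and opens its exit once enough attack balls are in a container.
; Player overlap with LockBox snaps EntryDoor1 to a fixed relative position.
; ContainerTrigger overlaps raise and lower the ball count, printing it for debugging.
; While the count is at least four, Tick lowers ExitDoor in small per-frame steps until it reaches a floor height.
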(event OnComponentBeginOverlap(LockBox)
  (params (OverlappedComponent :type Primitive%20Component%20Object%20Reference) (OtherActor :type Actor%20Object%20Reference) (OtherComp :type Primitive%20Component%20Object%20Reference) (OtherBodyIndex :type Integer) (bFromSweep :type Boolean) (SweepResult :type Hit%20Result%20Structure%20%28by%20ref%29))
  ;[1 1 1] Lock Room on player entry
  (Utilities|Casting|CastToPlayer_Char_BP OtherActor)
  (Transformation|SetRelativeLocation (Variables|Default|GetEntry%20door1) (Math|Vector|MakeVector -508.0 0.0 333.0) false false))

(event OnComponentBeginOverlap(ContainerTrigger)
  (params (OverlappedComponent :type Primitive%20Component%20Object%20Reference) (OtherActor :type Actor%20Object%20Reference) (OtherComp :type Primitive%20Component%20Object%20Reference) (OtherBodyIndex :type Integer) (bFromSweep :type Boolean) (SweepResult :type Hit%20Result%20Structure%20%28by%20ref%29))
  (bind _exit_door (Variables|Default|GetExit%20door))
  (bind _returnvalue (Transformation|GetWorldLocation _exit_door))
  (bind (_x _y _z) (Math|Vector|BreakVector _returnvalue))
  ;[1 1 1] Add one to counter when ball enter container
  (Utilities|Casting|CastToAttackBall_Bp OtherActor)
  (bind _output_get (Variables|Default|SetNumber%20of%20balls%20in%20container (+ (Variables|Default|GetNumber%20of%20balls%20in%20container) 1)))
  (Development|PrintString (Utilities|String|ToString(Integer) _output_get) true true "(R=0.000000,G=0.660000,B=1.000000,A=1.000000)" 5.0)
  (if (>= (Variables|Default|GetNumber%20of%20balls%20in%20container) 4)
    (if (not (< _z -3.8e+02))
      (Transformation|SetWorldLocation _exit_door (Math|Vector|MakeVector _x _y (- _z 1.0)) false false))))

(event OnComponentEndOverlap(ContainerTrigger)
  (params (OverlappedComponent :type Primitive%20Component%20Object%20Reference) (OtherActor :type Actor%20Object%20Reference) (OtherComp :type Primitive%20Component%20Object%20Reference) (OtherBodyIndex :type Integer))
  ;[1 1 1] Add one to counter when ball enter container
  (Utilities|Casting|CastToAttackBall_Bp OtherActor)
  (bind _output_get (Variables|Default|SetNumber%20of%20balls%20in%20container (- (Variables|Default|GetNumber%20of%20balls%20in%20container) 1)))
  (if (not (<= (Variables|Default|GetNumber%20of%20balls%20in%20container) 0))
    (Development|PrintString (Utilities|String|ToString(Integer) _output_get) true true "(R=0.000000,G=0.660000,B=1.000000,A=1.000000)" 5.0)))

(event EventTick
  (params (DeltaSeconds :type Float%20%28single-precision%29))
  (bind _exit_door (Variables|Default|GetExit%20door))
  (bind _returnvalue (Transformation|GetWorldLocation _exit_door))
  (bind (_x _y _z) (Math|Vector|BreakVector _returnvalue))
  (if (>= (Variables|Default|GetNumber%20of%20balls%20in%20container) 4)
    (if (not (< _z -3.8e+02))
      (Transformation|SetWorldLocation _exit_door (Math|Vector|MakeVector _x _y (- _z 1.0)) false false))))

(fn ConstructionScript)