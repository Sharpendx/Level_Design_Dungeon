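; Checkpoint actor that saves the player's position and rotation on overlap and restores them when play begins.
; A player overlapping its box deactivates all checkpoints, activates this one and records the transform.
; A second sequence branch, not gated by the player cast, writes that transform to the "Checkpoint" save slot.
; BeginPlay moves the player to any saved transform, while Tick swaps the light material to show active state.
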(event OnComponentBeginOverlap(Box)
  (params (OverlappedComponent :type Primitive%20Component%20Object%20Reference) (OtherActor :type Actor%20Object%20Reference) (OtherComp :type Primitive%20Component%20Object%20Reference) (OtherBodyIndex :type Integer) (bFromSweep :type Boolean) (SweepResult :type Hit%20Result%20Structure%20%28by%20ref%29))
  (Utilities|FlowControl|Sequence
    (:then_0
      ;[1 1 1] Update all checkpoints to newest one active and store the player's location & rotation when triggered
      (bind _asplayer_char_bp (Utilities|Casting|CastToPlayer_Char_BP OtherActor))
      (bind _outactors (Actor|GetAllActorsOfClass "CheckPoint_BP_C"))
      (for _array_element _outactors
        (bind _ascheck_point_bp (Utilities|Casting|CastToCheckPoint_BP _array_element))
        (Variables|CheckPoint_BP_C|SetIsActive _ascheck_point_bp false)
        (Variables|Default|SetIsActive true)
        (Variables|Default|SetPlayer%20Location (Transformation|GetActorLocation _asplayer_char_bp))
        (Variables|Default|SetPlayer%20Rotation (Transformation|GetActorRotation _asplayer_char_bp))))
    (:then_1
      ;[1 1 1] Ask if save of the game exists
      (bind _returnvalue (SaveGame|DoesSaveGameExist "Checkpoint"))
      (if _returnvalue
        ;[1 1 1] If yes, save the player's location
        (bind _returnvalue_2 (SaveGame|LoadGamefromSlot "Checkpoint"))
        (bind _ascheckpoint (Utilities|Casting|CastToCheckpoint _returnvalue_2))
        (Variables|/Game/Saves/Checkpoint.Checkpoint_C|SetPlayerLocationSave _ascheckpoint (Variables|Default|GetPlayer%20Location))
        (Variables|/Game/Saves/Checkpoint.Checkpoint_C|SetPlayerRotationSave _ascheckpoint (Variables|Default|GetPlayer%20Rotation))
        (SaveGame|SaveGametoSlot _ascheckpoint "Checkpoint")
        (else
          ;[1 1 1] If no, create a save and save the player location to it
          (bind _returnvalue_3 (SaveGame|CreateSaveGameObject "/Game/Saves/Checkpoint.Checkpoint_C"))
          (Variables|/Game/Saves/Checkpoint.Checkpoint_C|SetPlayerLocationSave _returnvalue_3 (Variables|Default|GetPlayer%20Location))
          (Variables|/Game/Saves/Checkpoint.Checkpoint_C|SetPlayerRotationSave _returnvalue_3 (Variables|Default|GetPlayer%20Rotation))
          (SaveGame|SaveGametoSlot _returnvalue_3 "Checkpoint")))
      (Development|PrintString "Checkpoint Saved"))))

(event EventBeginPlay
  (bind _returnvalue (SaveGame|DoesSaveGameExist "Checkpoint"))
  (if _returnvalue
    (bind _returnvalue_2 (SaveGame|LoadGamefromSlot "Checkpoint"))
    (bind _ascheckpoint (Utilities|Casting|CastToCheckpoint _returnvalue_2))
    (bind _asplayer_char_bp (Utilities|Casting|CastToPlayer_Char_BP (Game|GetPlayerCharacter 0)))
    (Transformation|SetActorLocation _asplayer_char_bp (Variables|/Game/Saves/Checkpoint.Checkpoint_C|GetPlayerLocationSave _ascheckpoint) false false)
    (Transformation|SetActorRotation _asplayer_char_bp (Variables|/Game/Saves/Checkpoint.Checkpoint_C|GetPlayerRotationSave _ascheckpoint))))

(event EventTick
  (params (DeltaSeconds :type Float%20%28single-precision%29))
  (bind _active_light (Variables|Default|GetActive%20Light))
  ;[1 1 1] Change color of Active Light based on if check point is active
  (if (Variables|Default|GetIsActive)
    (Rendering|Material|SetMaterial _active_light 0 "/Game/Materials/Plutonium.Plutonium")
    (else
      (Rendering|Material|SetMaterial _active_light 0 "/Game/Materials/M_TeleportEnemy.M_TeleportEnemy"))))

(fn ConstructionScript)