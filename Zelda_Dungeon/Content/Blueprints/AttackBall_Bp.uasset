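; AttackBall_Bp is a physics ball that hovers and shoots at the player within its trigger sphere.
; Player overlap disables gravity and adds a one-off upward force; leaving restores gravity, with PlayerDetected inverted (false means in range).
; While the flag is false, Tick faces the player and a five-second Delay paces Bullete_BP shots.
; Each shot launches forward from ProjectileSpawnLocation with a recoil impulse on the ball.
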(event OnComponentBeginOverlap(Sphere)
  (params (OverlappedComponent :type Primitive%20Component%20Object%20Reference) (OtherActor :type Actor%20Object%20Reference) (OtherComp :type Primitive%20Component%20Object%20Reference) (OtherBodyIndex :type Integer) (bFromSweep :type Boolean) (SweepResult :type Hit%20Result%20Structure%20%28by%20ref%29))
  (bind _staticmeshcomponent (Variables|Debug|GetStaticMeshComponent))
  ;[1 1 1] Turns off gravity when player is within the radius, renables when they are back in
  (Utilities|Casting|CastToPlayer_Char_BP OtherActor)
  (Variables|Default|SetPlayerDetected false)
  (Physics|SetEnableGravity _staticmeshcomponent (Variables|Default|GetPlayerDetected))
  ;[1 1 1] Make object slowly assend when withing radius
  (if (not (Variables|Default|GetPlayerDetected))
    (Physics|AddForce _staticmeshcomponent "0, 0,100000.000000" "None" false)))

(event OnComponentEndOverlap(Sphere)
  (params (OverlappedComponent :type Primitive%20Component%20Object%20Reference) (OtherActor :type Actor%20Object%20Reference) (OtherComp :type Primitive%20Component%20Object%20Reference) (OtherBodyIndex :type Integer))
  (bind _staticmeshcomponent (Variables|Debug|GetStaticMeshComponent))
  ;[1 1 1] Turns off gravity when player is within the radius, renables when they are back in
  (Utilities|Casting|CastToPlayer_Char_BP OtherActor)
  (Variables|Default|SetPlayerDetected true)
  (Physics|SetEnableGravity _staticmeshcomponent (Variables|Default|GetPlayerDetected))
  ;[1 1 1] Make object slowly assend when withing radius
  (if (not (Variables|Default|GetPlayerDetected))
    (Physics|AddForce _staticmeshcomponent "0, 0,100000.000000" "None" false)))

(event EventTick
  (params (DeltaSeconds :type Float%20%28single-precision%29))
  (bind _staticmeshcomponent (Variables|Debug|GetStaticMeshComponent))
  ;[1 1 1] Look at player code when in radius
  (if (not (Variables|Default|GetPlayerDetected))
    (Transformation|SetActorRotation (Math|Rotator|FindLookatRotation (Transformation|GetActorLocation) (Transformation|GetActorLocation (Game|GetPlayerCharacter 0))))
    ;[1 1 1] Fire a projectile after (x) seconds
    (Utilities|FlowControl|Delay 5.0)
    (if (not (Variables|Default|GetPlayerDetected))
      (bind _returnvalue (Game|SpawnActorfromClass "/Game/Blueprints/Bullete_BP.Bullete_BP_C" (Transformation|GetWorldTransform (Variables|Default|GetProjectile%20Spawn%20Location)) "Undefined" 0 0))
      (Physics|AddImpulse (Variables|/Game/Blueprints/Bullete_BP.Bullete_BP_C|GetBullet _returnvalue) (* (Math|Vector|GetForwardVector (Variables|Debug|GetStaticMeshComponent)) (Variables|Default|GetShootForce)) "None" true)
      (Physics|AddImpulse _staticmeshcomponent (* (Math|Vector|GetForwardVector _staticmeshcomponent) -1e+03) "None" true))))

(fn ConstructionScript)