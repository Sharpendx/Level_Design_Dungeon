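; CentralBrain is a boss-like AI actor that attacks the player once its trigger box is overlapped.
; Overlapping Box1 permanently sets PlayerInRoom, letting Tick use delays to repeatedly spawn a random NPC, explosion or attack ball beside the player.
; Each spawn is destroyed after a short delay.
; Any damage reduces Health by a fixed step, and the game quits after a delay once Health is depleted.
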(event OnComponentBeginOverlap(Box1)
  (params (OverlappedComponent :type Primitive%20Component%20Object%20Reference) (OtherActor :type Actor%20Object%20Reference) (OtherComp :type Primitive%20Component%20Object%20Reference) (OtherBodyIndex :type Integer) (bFromSweep :type Boolean) (SweepResult :type Hit%20Result%20Structure%20%28by%20ref%29))
  (Variables|Default|Setplayer%20in%20room true))

(event EventTick
  (params (DeltaSeconds :type Float%20%28single-precision%29))
  (bind _returnvalue (Game|GetPlayerCharacter 0))
  (bind _returnvalue_2 (Transformation|GetActorTransform _returnvalue))
  (bind _returnvalue_3 (+ (.location _returnvalue_2) "50.000000, 0, 0"))
  (bind _returnvalue_4 (Math|Transform|MakeTransform _returnvalue_3 (.rotation _returnvalue_2) (.scale _returnvalue_2)))
  (if (Variables|Default|Getplayer%20in%20room)
    (Utilities|FlowControl|Delay 2.0)
    (switch int (Math|Random|RandomIntegerinRange 0 2)
      (:0
        (bind _returnvalue_5 (AI|SpawnAIFromClass "/Game/Blueprints/AI/NPC.NPC_C" "/Game/Blueprints/AI/NPC_BT.NPC_BT" (+ (Transformation|GetActorLocation _returnvalue) "50.000000, 0, 0") "0, 0, 0" false))
        (Utilities|FlowControl|Delay 5.0)
        (Actor|DestroyActor _returnvalue_5))
      (:1
        (bind _returnvalue_6 (Game|SpawnActorfromClass "/Game/Blueprints/Explosion.Explosion_C" _returnvalue_4 "Undefined" 0 0))
        (Utilities|FlowControl|Delay 5.0)
        (Actor|DestroyActor _returnvalue_6))
      (:2
        (bind _returnvalue_7 (Game|SpawnActorfromClass "/Game/Blueprints/AttackBall_Bp.AttackBall_Bp_C" _returnvalue_4 "Undefined" 0 0))
        (Utilities|FlowControl|Delay 5.0)
        (Actor|DestroyActor _returnvalue_7)))))

(event Game|Damage|EventAnyDamage
  (params (Damage :type Float%20%28single-precision%29) (DamageType :type Damage%20Type%20Object%20Reference) (InstigatedBy :type Controller%20Object%20Reference) (DamageCauser :type Actor%20Object%20Reference))
  (Variables|Default|SetHealth (- (Variables|Default|GetHealth) 0.1))
  (Development|PrintString "Brain Has Taken Damage")
  (Utilities|FlowControl|Delay 3.0)
  (if (<= (Variables|Default|GetHealth) 0.0)
    (Game|QuitGame 0 "Quit" false)))

(fn ConstructionScript)