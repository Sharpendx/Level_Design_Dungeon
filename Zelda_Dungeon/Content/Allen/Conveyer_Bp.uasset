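; Conveyor Blueprint that carries any actor inside its Box volume along the conveyor's forward direction.
; Each Tick, it offsets every overlapping actor by the forward vector times Unitsseconds and delta time, giving a frame-rate-independent speed.
; The offset is applied without sweep, so moved actors are not stopped by blocking collision.
; The construction script resets the Arrow's world scale to one, keeping it unaffected by actor scaling.
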(event EventTick
  (params (DeltaSeconds :type Float%20%28single-precision%29))
  ;[1 1 1] On tick, add location to actors in zone
  (for _array_element (Collision|GetOverlappingActors (Variables|Default|GetBox) 0 :!class /Script/Engine.PrimitiveComponent)
    (Transformation|AddActorWorldOffset _array_element (* (Transformation|GetActorForwardVector) (* DeltaSeconds (Variables|Default|GetUnits/seconds))))))

(fn ConstructionScript
  ;[1 1 1] rescale arrow
  (Transformation|SetWorldScale3D (Variables|Default|GetArrow) "1.000000,1.000000,1.000000"))